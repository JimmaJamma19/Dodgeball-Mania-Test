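; BP_Thunder is a sprint power-up that sets an overlapping Player's FirstPersonCharacter SprintTime, then teleports to a random spot.
; MovinMulti calls MovingandSpawning, which checks GameManager_Blueprint's MatchTimer: at or above the threshold, the player's Red tag picks the X range.
; Below it, or on non-Player overlaps, a constant always-false comparison forces the non-Red X range with narrower Y.
; Tick plays its ActorSequence every frame.
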(event `self.Cube.OnComponentBeginOverlap`
  (params (OverlappedComponent :type "PrimitiveComponent Object Reference") (OtherActor :type "Actor Object Reference") (OtherComp :type "PrimitiveComponent Object Reference") (OtherBodyIndex :type Integer) (bFromSweep :type Boolean) (SweepResult :type "HitResult Structure (by ref)"))
  (bind _output_get (set `self.Actor Reference` OtherActor))
  (if (`self.ActorHasTag` "Player")
    (bind _asfirst_person_character (cast `/Game/Blueprints/FirstPersonCharacter` _output_get))
    (set `/Game/Blueprints/FirstPersonCharacter.SprintTime` 3.0 _asfirst_person_character)
    (`self.MovinMulti`)
    (else
      (if (< 0.0 -333.0) :!label _label
        (`self.K2_SetActorLocation` (`KismetMathLibrary.MakeVector` (`KismetMathLibrary.RandomFloatInRange` -2000.0 -500.0) (`KismetMathLibrary.RandomFloatInRange` 3700.0 5200.0) 130.0) false true)
        (else
          (`self.K2_SetActorLocation` (`KismetMathLibrary.MakeVector` (`KismetMathLibrary.RandomFloatInRange` -127.0 1300.0) (`KismetMathLibrary.RandomFloatInRange` 3700.0 5200.0) 130.0) false true))))))

(event `self.ReceiveTick`
  (params (DeltaSeconds :type "Float (single-precision)"))
  (`MovieSceneSequencePlayer.Play` (`ActorSequenceComponent.SequencePlayer` (`self.ActorSequence`))))

(event `MovinMulti`
  (`self.Moving and Spawning`))

(event `Moving and Spawning`
  (bind _returnvalue (`KismetMathLibrary.RandomFloatInRange` 2700.0 6200.0))
  (bind _returnvalue_2 (`GameplayStatics.GetActorOfClass` "/Game/Blueprints/GameManager_Blueprint.GameManager_Blueprint_C"))
  (if (< (`/Game/Blueprints/GameManager_Blueprint.MatchTimer` _returnvalue_2) 297.0)
    (goto _label)
    (elif (`self.ActorHasTag` (`self.Actor Reference`) "Red")
      (`self.K2_SetActorLocation` (`KismetMathLibrary.MakeVector` (`KismetMathLibrary.RandomFloatInRange` -2000.0 -500.0) _returnvalue 130.0) false true)
      (else
        (`self.K2_SetActorLocation` (`KismetMathLibrary.MakeVector` (`KismetMathLibrary.RandomFloatInRange` -127.0 1300.0) _returnvalue 130.0) false true)))))

(fn `UserConstructionScript`)