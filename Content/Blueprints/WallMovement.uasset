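; WallMovement is a wall actor that stays hidden at match start, then appears and slides sideways once the GameManager's MatchTimer drops below 150.
; Tick polls the manager and eases the Cube component along relative X, with the "Left" actor tag choosing the direction.
; After the move, it either sets FinishMove if the match is InProgress or resets the cube.
; A ResetPos event also restores the cube's relative transform.
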(event `self.ReceiveBeginPlay`
  (`SceneComponent.SetVisibility` (`self.Cube`) false false))

(event `self.ReceiveTick`
  (params (DeltaSeconds :type "Float (single-precision)"))
  (bind _cube (`self.Cube`))
  (bind (_returnvalue_x _returnvalue_y _returnvalue_z) (`KismetMathLibrary.BreakVector` (`SceneComponent.GetForwardVector` (`self.Cube`))))
  (bind (_returnvalue_x_2 _returnvalue_y_2 _returnvalue_z_2) (`KismetMathLibrary.BreakVector` (`SceneComponent.GetForwardVector` (`self.Cube`))))
  (bind _returnvalue (`GameplayStatics.GetActorOfClass` "/Game/Blueprints/GameManager_Blueprint.GameManager_Blueprint_C"))
  (if (< (`/Game/Blueprints/GameManager_Blueprint.MatchTimer` _returnvalue) 150.0)
    (`SceneComponent.SetVisibility` _cube true false)
    (set `self.OriginalPos` (`SceneComponent.RelativeLocation` _cube))
    (if (`self.ActorHasTag` self "Left")
      (`KismetSystemLibrary.MoveComponentTo` (`self.Cube`) (`KismetMathLibrary.MakeVector` (+ _returnvalue_x 666.0) _returnvalue_y _returnvalue_z) (struct) true true 5.0)
      (else
        (`KismetSystemLibrary.MoveComponentTo` (`self.Cube`) (`KismetMathLibrary.MakeVector` (- _returnvalue_x_2 666.0) _returnvalue_y_2 _returnvalue_z_2) (struct) true true 5.0)))
    (bind _returnvalue_2 (`GameplayStatics.GetActorOfClass` "/Game/Blueprints/GameManager_Blueprint.GameManager_Blueprint_C"))
    (if (`/Game/Blueprints/GameManager_Blueprint.InProgress` _returnvalue_2)
      (set `self.FinishMove` true)
      (else
        (`SceneComponent.ResetRelativeTransform` (`self.Cube`))))))

(event `ResetPos`
  (`SceneComponent.ResetRelativeTransform` (`self.Cube`)))

(fn `UserConstructionScript`)