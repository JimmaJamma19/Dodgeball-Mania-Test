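; Game manager Blueprint for a Red-versus-Blue ball match, tracking teams, eliminations and the match timer.
; Server events build rosters from actor tags, move eliminated players to out lists and reveal that team's TM8 target.
; An empty roster or expired timer triggers Reset, which scatters players, strips their last tag and restores abilities and walls.
; The win check announces the emptied team as winner; OutBlue/OutRed events are unwired stubs.
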(event `OutBlue`
  (params (NewBlueOut :type "Actor Object Reference (by ref)")))

(event `OutRed`
  (params (NewRedOut :type "Actor Object Reference (by ref)")))

(event `OutBlueMulti`
  (params (NewBlueOut :type "Actor Object Reference (by ref)")))

(event `OutRedMulti`
  (params (NewRedOut :type "Actor Object Reference (by ref)")))

(event `OutBlueServer`
  (params (NewBlueOut :type "Actor Object Reference (by ref)")))

(event `OutRedServer`
  (params (NewRedOut :type "Actor Object Reference (by ref)")))

(event `TeamCountServer`
  (`self.TeamCount`))

(event `TeamCount`
  (bind _outactors (`GameplayStatics.GetAllActorsWithTag` "Blue"))
  (bind _output_get (set `self.BlueTeam` _outactors))
  (bind _outactors_2 (`GameplayStatics.GetAllActorsWithTag` "Red"))
  (bind _output_get_2 (set `self.RedTeam` _outactors_2))
  (set `self.InitalRedTeam` (`KismetArrayLibrary.Array_Length` _output_get_2))
  (set `self.InitialBlueTeam` (`KismetArrayLibrary.Array_Length` _output_get)))

(event `Update Teams`
  (params (`Actor Reference` :type "Actor Object Reference"))
  (`self.Update Teams Server` `Actor Reference`))

(event `Update Teams Server`
  (params (`Actor Reference` :type "Actor Object Reference"))
  (bind _actor_reference (`self.Actor Reference`))
  (bind _actor_reference_2 (`self.Actor Reference`))
  (bind _output_get (set `self.Actor Reference` `Actor Reference`))
  (if (`self.ActorHasTag` _output_get "Red")
    (`KismetArrayLibrary.Array_RemoveItem` (`self.RedTeam`) _actor_reference_2)
    (`KismetArrayLibrary.Array_Add` (`self.OutRedTeam`) _actor_reference_2)
    (bind _returnvalue (`GameplayStatics.GetActorOfClass` "/Game/Blueprints/RedTM8Target.RedTM8Target_C"))
    (`/Game/Blueprints/RedTM8Target.MakeVisibleMulti` _returnvalue)
    (else
      (`KismetArrayLibrary.Array_RemoveItem` (`self.BlueTeam`) _actor_reference)
      (`KismetArrayLibrary.Array_Add` (`self.OutBlueTeam`) _actor_reference)
      (bind _returnvalue_2 (`GameplayStatics.GetActorOfClass` "/Game/Blueprints/BlueTM8Target.BlueTM8Target_C"))
      (`/Game/Blueprints/BlueTM8Target.MakeVisibleMulti` _returnvalue_2))))

(event `CheckGameStateServer`
  (`self.CheckGameState`))

(event `CheckGameState`
  (if (or (<= (`KismetArrayLibrary.Array_Length` (`self.BlueTeam`)) 0) (<= (`KismetArrayLibrary.Array_Length` (`self.RedTeam`)) 0))
    (if (<= (`KismetArrayLibrary.Array_Length` (`self.RedTeam`)) 0)
      (set `self.WinningTeam` 1)
      (`KismetSystemLibrary.PrintString` "Red Team wins" true true (struct :`R` 0.144125 :`G` 1.0 :`A` 1.0) 10.0)
      (else
        (set `self.WinningTeam` 2)
        (`KismetSystemLibrary.PrintString` "Blue Team wins" true true (struct :`R` 0.144125 :`G` 1.0 :`A` 1.0) 10.0)))
    (`self.Reset`)))

(event `self.ReceiveTick`
  (params (DeltaSeconds :type "Float (single-precision)"))
  (set `self.Delta Seconds` DeltaSeconds)
  (if (`self.InProgress`)
    (if (> (`self.MatchTimer`) 0.0)
      (set `self.MatchTimer` (- (`self.MatchTimer`) (`self.Delta Seconds`)))
      (else
        (`self.Reset`)))))

(event `Reset`
  (set `self.InProgress` false)
  (set `self.MatchTimer` 300.0)
  (bind _outactors (`GameplayStatics.GetAllActorsWithTag` "Player"))
  (for _array_element _outactors
    (`self.K2_SetActorLocation` _array_element (`KismetMathLibrary.MakeVector` (`KismetMathLibrary.RandomFloatInRange` -863.0 850.0) (`KismetMathLibrary.RandomFloatInRange` 1900.0 3000.0) 500.0) false true)
    (bind _tags (`Actor.Tags` _array_element))
    (`KismetArrayLibrary.Array_Remove` _tags (`KismetArrayLibrary.Array_LastIndex` _tags))
    (bind _asfirst_person_character (cast `/Game/Blueprints/FirstPersonCharacter` _array_element))
    (`SceneComponent.SetVisibility` (`/Game/Blueprints/FirstPersonCharacter.Ball_Hold_holder` _asfirst_person_character) false false)
    (set `/Game/Blueprints/FirstPersonCharacter.SprintTime` 3.0 _asfirst_person_character)
    (set `/Game/Blueprints/FirstPersonCharacter.DodgeNumbers` 3 _asfirst_person_character))
  (`KismetArrayLibrary.Array_Clear` (`self.BlueTeam`))
  (`KismetArrayLibrary.Array_Clear` (`self.OutRedTeam`))
  (`KismetArrayLibrary.Array_Clear` (`self.OutBlueTeam`))
  (`KismetArrayLibrary.Array_Clear` (`self.RedTeam`))
  (set `self.InitalRedTeam` 0)
  (set `self.InitialBlueTeam` 0)
  (bind _outactors_2 (`GameplayStatics.GetAllActorsOfClass` "/Game/Blueprints/WallMovement.WallMovement_C"))
  (for _array_element_2 _outactors_2
    (`SceneComponent.SetVisibility` (`/Game/Blueprints/WallMovement.Cube` _array_element_2) false false)
    (if (`/Game/Blueprints/WallMovement.FinishMove` _array_element_2)
      (`/Game/Blueprints/WallMovement.ResetPos` _array_element_2))))

(fn `UserConstructionScript`)