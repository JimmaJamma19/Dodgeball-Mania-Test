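; Blue team target that brings sidelined players back into play when hit by an actor tagged Ball.
; A hit teleports a random OutBlueTeam player, resets sprint and dodges, and shifts them to BlueTeam on GameManager_Blueprint, re-rolling the random pick at each step.
; It starts hidden, DisplayCheck shows it while OutBlueTeam has players, and a hit that empties that list hides it.
; Overlapping Walls relocates it randomly.
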(event `MakeVisibleMulti`
  (`self.MakeVisible`))

(event `HideMulti`
  (`self.Hide`))

(event `MakeVisible`
  (`SceneComponent.SetVisibility` (`self.Target`) true false))

(event `Hide`
  (`SceneComponent.SetVisibility` (`self.Target`) false false :!label _label))

(event `self.ReceiveBeginPlay`
  (goto _label))

(event `self.Target.OnComponentHit`
  (params (HitComponent :type "PrimitiveComponent Object Reference") (OtherActor :type "Actor Object Reference") (OtherComp :type "PrimitiveComponent Object Reference") (NormalImpulse :type "Vector Structure") (Hit :type "HitResult Structure (by ref)"))
  (bind _output_get (set `self.ActorReference` OtherActor))
  (if (`self.ActorHasTag` _output_get "Ball")
    (bind _returnvalue (`GameplayStatics.GetActorOfClass` "/Game/Blueprints/GameManager_Blueprint.GameManager_Blueprint_C"))
    (bind _asgame_manager_blueprint (cast `/Game/Blueprints/GameManager_Blueprint` _returnvalue))
    (bind _outblueteam (`/Game/Blueprints/GameManager_Blueprint.OutBlueTeam` _asgame_manager_blueprint))
    (bind _outitem (`KismetArrayLibrary.Array_Random` _outblueteam))
    (`self.K2_SetActorLocation` _outitem (`KismetMathLibrary.MakeVector` (`KismetMathLibrary.RandomFloatInRange` -900.0 870.0) -2650.0 80.0) false true)
    (bind _asfirst_person_character (cast `/Game/Blueprints/FirstPersonCharacter` _outitem))
    (set `/Game/Blueprints/FirstPersonCharacter.SprintTime` 3.0 _asfirst_person_character)
    (set `/Game/Blueprints/FirstPersonCharacter.DodgeNumbers` 3 _asfirst_person_character)
    (`KismetArrayLibrary.Array_RemoveItem` _outblueteam _outitem)
    (`KismetArrayLibrary.Array_Add` (`/Game/Blueprints/GameManager_Blueprint.BlueTeam` _asgame_manager_blueprint) _outitem)
    (if (== (`KismetArrayLibrary.Array_Length` _outblueteam) 0)
      (`self.HideMulti`)
      (`KismetSystemLibrary.PrintString` "Player Redeemed"))))

(event `self.Target.OnComponentBeginOverlap`
  (params (OverlappedComponent :type "PrimitiveComponent Object Reference") (OtherActor :type "Actor Object Reference") (OtherComp :type "PrimitiveComponent Object Reference") (OtherBodyIndex :type Integer) (bFromSweep :type Boolean) (SweepResult :type "HitResult Structure (by ref)"))
  (if (`self.ActorHasTag` OtherActor "Walls")
    (`self.K2_SetActorLocation` (`KismetMathLibrary.MakeVector` -2126.273438 (`KismetMathLibrary.RandomFloatInRange` 3700.0 5200.0) (`KismetMathLibrary.RandomFloatInRange` 500.0 900.0)) false true)))

(event `DisplayCheck`
  (bind _target (`self.Target`))
  (bind _returnvalue (`GameplayStatics.GetActorOfClass` "/Game/Blueprints/GameManager_Blueprint.GameManager_Blueprint_C"))
  (if (!= (`KismetArrayLibrary.Array_Length` (`/Game/Blueprints/GameManager_Blueprint.OutBlueTeam` _returnvalue)) 0)
    (`SceneComponent.SetVisibility` _target true false)
    (else
      (`SceneComponent.SetVisibility` _target false false))))

(fn `UserConstructionScript`)