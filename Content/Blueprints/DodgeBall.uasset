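; Dodgeball actor that eliminates players it hits while live and is picked up by empty-handed players otherwise.
; Mesh hits on players pass through a DoOnce into Multi wrapper events; other hits deaden the ball and reset the gate.
; Elimination teleports the player to a random spot, respawns balls above the hit location, including any held one, and updates GameManager_Blueprint.
; Older elimination, pickup and debug chains remain unreached.
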(event `self.StaticMeshComponent.OnComponentHit`
  (params (HitComponent :type "PrimitiveComponent Object Reference") (OtherActor :type "Actor Object Reference") (OtherComp :type "PrimitiveComponent Object Reference") (NormalImpulse :type "Vector Structure") (Hit :type "HitResult Structure (by ref)"))
  (bind _output_get (set `self.Actor Reference` OtherActor))
  (if (`self.LiveBall`)
    (`GameplayStatics.PlaySoundAtLocation` "/Game/dodgeball.dodgeball" (0.0 0.0 0.0) (struct) 1.0 1.0 0.0 null null null))
  (if (`self.ActorHasTag` _output_get "Player")
    (`/Engine/EditorBlueprintResources/StandardMacros.DoOnce` false :!label _label
      (:`Completed`
        (if (`self.LiveBall`)
          (set `self.LiveBall` false)
          (`self.EliminateMulti`)
          (`KismetSystemLibrary.PrintString` "Player Hit" true true (struct :`G` 0.66 :`B` 1.0 :`A` 1.0) 5.0)
          (else
            (`self.PickupMulti`)))))
    (else
      (set `self.LiveBall` false)
      (goto _label :!via `Reset`))))

(event `PickupMulti`
  (`self.Pickup`))

(event `Pickup`
  (bind _asfirst_person_character (cast `/Game/Blueprints/FirstPersonCharacter` (`self.Actor Reference`)))
  (if (not (`/Game/Blueprints/FirstPersonCharacter.Holding_Ball` _asfirst_person_character))
    (`/Game/Blueprints/FirstPersonCharacter.Ball in Hand` _asfirst_person_character)
    (`self.K2_DestroyActor`)
    (`KismetSystemLibrary.PrintString` "Player pickup" true true (struct :`G` 1.0 :`B` 0.096458 :`A` 1.0) 5.0)))

(event `BallSpawnMulti`
  (`self.BallSpawn`))

(event `BallSpawn`
  (bind _asfirst_person_character (cast `/Game/Blueprints/FirstPersonCharacter` (`self.Actor Reference`)))
  (if (`/Game/Blueprints/FirstPersonCharacter.Holding_Ball` _asfirst_person_character)
    (bind _returnvalue (`|SpawnActorFromClass` "DodgeBall_C" (`KismetMathLibrary.MakeTransform` (`KismetMathLibrary.MakeVector` (.x (`self.EliminatePos`)) (.y (`self.EliminatePos`)) (+ (.z (`self.EliminatePos`)) 400.0))) "Undefined" "OverrideRootScale" null null))
    (set `/Game/Blueprints/DodgeBall.LiveBall` false _returnvalue)
    (`/Game/Blueprints/FirstPersonCharacter.Ball in Hand` _asfirst_person_character)))

(event `EliminateMulti`
  (`self.Elimate`))

(event `Elimate`
  (bind _asfirst_person_character (cast `/Game/Blueprints/FirstPersonCharacter` (`self.Actor Reference`)))
  (set `self.EliminatePos` (`self.K2_GetActorLocation` _asfirst_person_character))
  (`self.K2_SetActorLocation` (`self.Actor Reference`) (`KismetMathLibrary.MakeVector` (`KismetMathLibrary.RandomFloatInRange` -863.0 850.0) (`KismetMathLibrary.RandomFloatInRange` 1900.0 3000.0) 500.0) false false)
  (`self.K2_DestroyActor`)
  (`self.BallSpawnMulti`)
  (bind _returnvalue (`GameplayStatics.GetActorOfClass` "/Game/Blueprints/GameManager_Blueprint.GameManager_Blueprint_C"))
  (bind _asgame_manager_blueprint (cast `/Game/Blueprints/GameManager_Blueprint` _returnvalue))
  (`/Game/Blueprints/GameManager_Blueprint.Update Teams` _asgame_manager_blueprint (`self.Actor Reference`))
  (`/Game/Blueprints/GameManager_Blueprint.CheckGameStateServer` _asgame_manager_blueprint)
  (`|SpawnActorFromClass` "DodgeBall_C" (`KismetMathLibrary.MakeTransform` (`KismetMathLibrary.MakeVector` (.x (`self.EliminatePos`)) (.y (`self.EliminatePos`)) (+ (.z (`self.EliminatePos`)) 400.0))) "Undefined" "OverrideRootScale" null null))

(event `Eliminate`
  (if (`self.ActorHasTag` (`self.Actor Reference`) "Walls")
    (set `self.LiveBall` false)
    (elif (`self.ActorHasTag` (`self.Actor Reference`) "Player")
      (set `self.LiveBall` false)
      (`KismetSystemLibrary.PrintString` "Player has been elimated" true true (struct :`R` 1.0 :`B` 0.987626 :`A` 1.0) 5.0)
      (bind _asfirst_person_character (cast `/Game/Blueprints/FirstPersonCharacter` (`self.Actor Reference`)))
      (`/Game/Blueprints/FirstPersonCharacter.PlayerOut` _asfirst_person_character)
      (`self.UpdatePlayerCount`)
      (`self.OutArrayUpdate`))))

(event `OutArrayUpdate`
  (bind _actor_reference (`self.Actor Reference`))
  (bind _game_manager (`self.Game Manager`))
  (if (`self.ActorHasTag` _actor_reference "Blue")
    (`/Game/Blueprints/GameManager_Blueprint.OutBlue` _game_manager _actor_reference)
    (else
      (`/Game/Blueprints/GameManager_Blueprint.OutRed` _game_manager _actor_reference))))

(event `PickupBall`
  (if (`self.ActorHasTag` (`self.Actor Reference`) "Player")
    (bind _asfirst_person_character (cast `/Game/Blueprints/FirstPersonCharacter` (`self.Actor Reference`)))
    (if (not (`/Game/Blueprints/FirstPersonCharacter.Holding_Ball` _asfirst_person_character))
      (`/Game/Blueprints/FirstPersonCharacter.Ball in Hand` _asfirst_person_character)
      (`PrimitiveComponent.SetOnlyOwnerSee` (`/Game/Blueprints/FirstPersonCharacter.Ball_Hold_holder` _asfirst_person_character) false)
      (`self.K2_DestroyActor`)
      (`KismetSystemLibrary.PrintString` "Player can/has picked up ball" true true (struct :`R` 1.0 :`G` 0.861521 :`A` 1.0) 5.0))))

(event `UpdatePlayerCount`
  (bind _actor_reference (`self.Actor Reference`))
  (bind _actor_reference_2 (`self.Actor Reference`))
  (bind _game_manager (`self.Game Manager`))
  (bind _returnvalue (`GameplayStatics.GetActorOfClass` "/Game/Blueprints/GameManager_Blueprint.GameManager_Blueprint_C"))
  (bind _asgame_manager_blueprint (cast `/Game/Blueprints/GameManager_Blueprint` _returnvalue))
  (set `self.Game Manager` _asgame_manager_blueprint)
  (if (`self.ActorHasTag` _actor_reference_2 "Blue")
    (`KismetArrayLibrary.Array_RemoveItem` (`/Game/Blueprints/GameManager_Blueprint.BlueTeam` _game_manager) _actor_reference)
    (`KismetArrayLibrary.Array_Add` (`/Game/Blueprints/GameManager_Blueprint.OutBlueTeam` _game_manager) _actor_reference)
    (elif (`self.ActorHasTag` _actor_reference_2 "Red")
      (`KismetArrayLibrary.Array_RemoveItem` (`/Game/Blueprints/GameManager_Blueprint.RedTeam` _game_manager) _actor_reference)
      (`KismetArrayLibrary.Array_Add` (`/Game/Blueprints/GameManager_Blueprint.OutRedTeam` _game_manager) _actor_reference))))

(fn `UserConstructionScript`)