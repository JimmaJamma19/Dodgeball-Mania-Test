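; Spinning pickup that grants an overlapping Player-tagged FirstPersonCharacter an extra dodge charge, up to a cap of three.
; After a grant, MovinMulti calls MovingandSpawning, which checks the GameManager match timer.
; Early in the match it teleports to a random spot chosen by the collector's Red tag.
; Later, or on non-player overlap, it relocates randomly within one of two zones chosen by its current Y.
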(event `self.Cube.OnComponentBeginOverlap`
  (params (OverlappedComponent :type "PrimitiveComponent Object Reference") (OtherActor :type "Actor Object Reference") (OtherComp :type "PrimitiveComponent Object Reference") (OtherBodyIndex :type Integer) (bFromSweep :type Boolean) (SweepResult :type "HitResult Structure (by ref)"))
  (bind (_returnvalue_x _returnvalue_y) (`KismetMathLibrary.BreakVector` (`SceneComponent.K2_GetComponentLocation` (`self.Cube`))))
  (bind _output_get (set `self.Actor Reference` OtherActor))
  (if (`self.ActorHasTag` _output_get "Player")
    (bind _asfirst_person_character (cast `/Game/Blueprints/FirstPersonCharacter` OtherActor))
    (bind _dodgenumbers (`/Game/Blueprints/FirstPersonCharacter.DodgeNumbers` _asfirst_person_character))
    (if (<= _dodgenumbers 2)
      (`/Engine/EditorBlueprintResources/StandardMacros.IncrementInt` _dodgenumbers
        (:`  `
          (`self.MovinMulti`))))
    (else
      (if (< _returnvalue_y -333.0) :!label _label
        (`self.K2_SetActorLocation` (`KismetMathLibrary.MakeVector` (`KismetMathLibrary.RandomFloatInRange` -870.0 840.0) (`KismetMathLibrary.RandomFloatInRange` -2600.0 -650.0) 30.0) false true)
        (else
          (`self.K2_SetActorLocation` (`KismetMathLibrary.MakeVector` (`KismetMathLibrary.RandomFloatInRange` -879.0 843.0) (`KismetMathLibrary.RandomFloatInRange` -387.0 1600.0) 30.0) false true))))))

(event `MovinMulti`
  (`self.MovingandSpawning`))

(event `MovingandSpawning`
  (bind _returnvalue (`KismetMathLibrary.RandomFloatInRange` 2700.0 6200.0))
  (bind _returnvalue_2 (`GameplayStatics.GetActorOfClass` "/Game/Blueprints/GameManager_Blueprint.GameManager_Blueprint_C"))
  (if (< (`/Game/Blueprints/GameManager_Blueprint.MatchTimer` _returnvalue_2) 150.0)
    (if (`self.ActorHasTag` (`self.Actor Reference`) "Red")
      (`self.K2_SetActorLocation` (`KismetMathLibrary.MakeVector` (`KismetMathLibrary.RandomFloatInRange` -2000.0 -500.0) _returnvalue 130.0) false true)
      (else
        (`self.K2_SetActorLocation` (`KismetMathLibrary.MakeVector` (`KismetMathLibrary.RandomFloatInRange` -127.0 1300.0) _returnvalue 130.0) false true)))
    (else
      (goto _label))))

(event `self.ReceiveTick`
  (params (DeltaSeconds :type "Float (single-precision)"))
  (`SceneComponent.K2_AddLocalRotation` (`self.Cube`) (`KismetMathLibrary.MakeRotator` 0.0 0.0 (* (`self.Rotator`) DeltaSeconds)) false false))

(fn `UserConstructionScript`)